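; Playable killer character that attacks survivors and can pick up those who have taken a second hit.
; Enhanced Input drives movement, look and a montage attack locked until completion, while Hit box-traces at the weapon socket and triggers the survivor's hit reaction.
; Survivor overlap events show a prompt and open a gate for the trigger input to attach the survivor to the Holding socket.
; Key 1 detaches the survivor found by class; hook logic is unwired.
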(event Custom|Evt_End%20Overlap%20Event%20Survivor
  (params (Survivor :type BP%20Survivorll%20Object%20Reference))
  (if (Variables|/Game/Create/GM/BP_Survivorll.BP_Survivorll_C|GetbSecondHit Survivor)
    (if (not (Variables|Default|GetGrabToSurvivor))
      (Utilities|IsValid (stale Custom|Evt_Begin%20Overlap%20Event%20Survivor _returnvalue)
        (:Is%20Valid
          (Widget|RemovefromParent (stale Custom|Evt_Begin%20Overlap%20Event%20Survivor _returnvalue))
          (Utilities|FlowControl|Gate true) ; enters at Close
        )))))

(event Custom|Evt_Begin%20Overlap%20Event%20Survivor
  (params (Survivor :type BP%20Survivorll%20Object%20Reference))
  (if (Variables|/Game/Create/GM/BP_Survivorll.BP_Survivorll_C|GetbSecondHit Survivor)
    (if (not (Variables|Default|GetGrabToSurvivor))
      (bind _returnvalue (UserInterface|CreateWidget "/Game/Create/Widget/WG_Trigger_Info.WG_Trigger_Info_C"))
      (UserInterface|Viewport|AddtoPlayerScreen _returnvalue)
      (Utilities|FlowControl|Gate true) ; enters at Open
    )))

(event Input|EnhancedActionEvents|EnhancedInputActionIA_Attack
  (params (ActionValue :type Boolean) (ElapsedSeconds :type Float%20%28double-precision%29) (TriggeredSeconds :type Float%20%28double-precision%29) (InputAction :type Input%20Action%20Object%20Reference :default "/Game/Create/GM/Input/Killer/IA_Attack.IA_Attack"))
  (Utilities|FlowControl|DoOnce false :!label _label
    (:Completed
      (Animation|Montage|PlayMontage (Variables|Character|GetMesh) "/Game/Create/Animation/Killer/Anim_Attack.Anim_Attack"
        (:OnCompleted
          (goto _label Reset))))))

(event Input|EnhancedActionEvents|EnhancedInputActionIA_Killer_Trigger
  (params (ActionValue :type Boolean) (ElapsedSeconds :type Float%20%28double-precision%29) (TriggeredSeconds :type Float%20%28double-precision%29) (InputAction :type Input%20Action%20Object%20Reference :default "/Game/Create/GM/Input/Killer/IA_Killer_Trigger.IA_Killer_Trigger"))
  (Utilities|FlowControl|Gate true
    (:Exit
      (Transformation|AttachComponentToComponent (stale Custom|Evt_Begin%20Overlap%20Event%20Survivor Survivor) (Variables|Character|GetMesh) "Holding" "SnapToTarget" "SnapToTarget" "SnapToTarget" true)
      (Collision|SetActorEnableCollision (stale Custom|Evt_Begin%20Overlap%20Event%20Survivor Survivor) false)
      (Widget|RemovefromParent (stale Custom|Evt_Begin%20Overlap%20Event%20Survivor _returnvalue))
      (Variables|Default|SetGrabToSurvivor true))))

(event Input|EnhancedActionEvents|EnhancedInputActionIA_Killer_Trigger
  (params (ActionValue :type Boolean) (ElapsedSeconds :type Float%20%28double-precision%29) (TriggeredSeconds :type Float%20%28double-precision%29) (InputAction :type Input%20Action%20Object%20Reference :default "/Game/Create/GM/Input/Killer/IA_Killer_Trigger.IA_Killer_Trigger")))

(event Input|EnhancedActionEvents|EnhancedInputActionIA_Look
  (params (ActionValue :type Vector%202D%20Structure) (ElapsedSeconds :type Float%20%28double-precision%29) (TriggeredSeconds :type Float%20%28double-precision%29) (InputAction :type Input%20Action%20Object%20Reference :default "/Game/Create/GM/Input/Actions/IA_Look.IA_Look"))
  ;[1 1 1] Camera
  (Pawn|Input|AddControllerYawInput (.x ActionValue))
  (Pawn|Input|AddControllerPitchInput (.y ActionValue)))

(event Input|EnhancedActionEvents|EnhancedInputActionIA_Move
  (params (ActionValue :type Vector%202D%20Structure) (ElapsedSeconds :type Float%20%28double-precision%29) (TriggeredSeconds :type Float%20%28double-precision%29) (InputAction :type Input%20Action%20Object%20Reference :default "/Game/Create/GM/Input/Actions/IA_Move.IA_Move"))
  (bind _returnvalue (Pawn|GetControlRotation :!class /Script/Engine.Pawn))
  ;[1 1 1] Movement
  (Pawn|Input|AddMovementInput (Math|Vector|GetRightVector (Math|Rotator|MakeRotator (.roll _returnvalue) 0.0 (.yaw _returnvalue))) (.x ActionValue) false)
  (Pawn|Input|AddMovementInput (Math|Vector|GetForwardVector (Math|Rotator|MakeRotator 0.0 0.0 (.yaw (Pawn|GetControlRotation :!class /Script/Engine.Pawn)))) (.y ActionValue) false))

(event EventBeginPlay
  ;[1 1 1] Input
  (bind _asplayer_controller (Utilities|Casting|CastToPlayerController (Pawn|GetController)))
  (Utilities|IsValid (PlayerController|LocalPlayerSubsystems|GetEnhancedInputLocalPlayerSubsystem _asplayer_controller)
    (:Is%20Valid
      (Input|AddMappingContext (PlayerController|LocalPlayerSubsystems|GetEnhancedInputLocalPlayerSubsystem _asplayer_controller) "/Game/Create/GM/Input/IMC_Killer.IMC_Killer" 0 "(bIgnoreAllPressedKeysUntilRelease=True,bForceImmediately=False,bNotifyUserSettings=False)"))))

(event Input|KeyboardEvents|1
  (params (Key :type Key%20Structure :default "None"))
  (:Pressed
    (bind _returnvalue (Actor|GetActorOfClass "/Game/Create/GM/BP_Survivorll.BP_Survivorll_C"))
    (Collision|SetActorEnableCollision _returnvalue true)
    (Default|Detach _returnvalue)))

(fn ConstructionScript
  (Transformation|AttachComponentToComponent (Variables|Default|GetWeapon) (Variables|Character|GetMesh) "Weapon_Hand" "SnapToTarget" "SnapToTarget" "SnapToTarget" true))

(fn Hit
  (bind _mesh (Variables|Character|GetMesh))
  (bind _returnvalue (Transformation|GetSocketLocation _mesh "Weapon_Hand"))
  (bind _outhit (Class|KismetSystemLibrary|BoxTraceSingleforObjects _returnvalue _returnvalue "5.000000,5.000000,5.000000" (Transformation|GetSocketRotation _mesh "Weapon_Hand") (Utilities|Array|MakeArray "ObjectTypeQuery3") false 0 "ForDuration" true))
  (bind _asbp_survivorll (Utilities|Casting|CastToBP_Survivorll (.HitActor (Collision|BreakHitResult _outhit))))
  (Animation|PlayAnimMontage "/Game/Create/Animation/Killer/Anim_Attack_Delay.Anim_Attack_Delay" 1.5 "None")
  (Default|HitMotion _asbp_survivorll))