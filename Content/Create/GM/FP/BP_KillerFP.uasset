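; BP_KillerFP is the first-person killer character, with Enhanced Input movement, look and attack montage, and a weapon attached to its hand socket.
; Hit box-traces for pawns at that socket and plays an attack delay montage when it strikes a survivor.
; Overlapping a survivor flagged SecondHit shows a trigger prompt widget and opens a gate for the trigger input, which has no connected action.
; Controller-call, carry-attach and hit-counting logic sit unconnected.
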(event OnComponentBeginOverlap(CapsuleComponent)
  (params (OverlappedComponent :type Primitive%20Component%20Object%20Reference) (OtherActor :type Actor%20Object%20Reference) (OtherComp :type Primitive%20Component%20Object%20Reference) (OtherBodyIndex :type Integer) (bFromSweep :type Boolean) (SweepResult :type Hit%20Result%20Structure%20%28by%20ref%29))
  (bind _asbp_survivorll (Utilities|Casting|CastToBP_Survivorll OtherActor))
  (if (Variables|/Game/Create/GM/BP_Survivorll.BP_Survivorll_C|GetbSecondHit _asbp_survivorll)
    (bind _returnvalue (UserInterface|CreateWidget "/Game/Create/Widget/WG_Trigger_Info.WG_Trigger_Info_C"))
    (UserInterface|Viewport|AddtoPlayerScreen _returnvalue)
    (Utilities|FlowControl|Gate true) ; enters at Open
  ))

(event Input|EnhancedActionEvents|EnhancedInputActionIA_Attack
  (params (ActionValue :type Boolean) (ElapsedSeconds :type Float%20%28double-precision%29) (TriggeredSeconds :type Float%20%28double-precision%29) (InputAction :type Input%20Action%20Object%20Reference :default "/Game/Create/GM/Input/Killer/IA_Attack.IA_Attack"))
  (Animation|Montage|PlayMontage (Variables|Character|GetMesh) "/Game/Create/Animation/KillerFP/Anim_Attack_FP.Anim_Attack_FP"))

(event Input|EnhancedActionEvents|EnhancedInputActionIA_Killer_Trigger
  (params (ActionValue :type Boolean) (ElapsedSeconds :type Float%20%28double-precision%29) (TriggeredSeconds :type Float%20%28double-precision%29) (InputAction :type Input%20Action%20Object%20Reference :default "/Game/Create/GM/Input/Killer/IA_Killer_Trigger.IA_Killer_Trigger"))
  (Utilities|FlowControl|Gate true))

(event Input|EnhancedActionEvents|EnhancedInputActionIA_Look
  (params (ActionValue :type Vector%202D%20Structure) (ElapsedSeconds :type Float%20%28double-precision%29) (TriggeredSeconds :type Float%20%28double-precision%29) (InputAction :type Input%20Action%20Object%20Reference :default "/Game/Create/GM/Input/Actions/IA_Look.IA_Look"))
  (Pawn|Input|AddControllerYawInput (.x ActionValue))
  (Pawn|Input|AddControllerPitchInput (.y ActionValue)))

(event Input|EnhancedActionEvents|EnhancedInputActionIA_Move
  (params (ActionValue :type Vector%202D%20Structure) (ElapsedSeconds :type Float%20%28double-precision%29) (TriggeredSeconds :type Float%20%28double-precision%29) (InputAction :type Input%20Action%20Object%20Reference :default "/Game/Create/GM/Input/Actions/IA_Move.IA_Move"))
  (bind _returnvalue (Pawn|GetControlRotation :!class /Script/Engine.Pawn))
  (Pawn|Input|AddMovementInput (Math|Vector|GetRightVector (Math|Rotator|MakeRotator (.roll _returnvalue) 0.0 (.yaw _returnvalue))) (.x ActionValue) false)
  (Pawn|Input|AddMovementInput (Math|Vector|GetForwardVector (Math|Rotator|MakeRotator 0.0 0.0 (.yaw (Pawn|GetControlRotation :!class /Script/Engine.Pawn)))) (.y ActionValue) false))

(event EventBeginPlay)

(fn ConstructionScript
  (Transformation|AttachComponentToComponent (Variables|Default|GetSM_Weapon) (Variables|Character|GetMesh) "Weapon_Hand" "SnapToTarget" "SnapToTarget" "SnapToTarget" true))

(fn Hit
  (bind _mesh (Variables|Character|GetMesh))
  (bind _returnvalue (Transformation|GetSocketLocation _mesh "Weapon_Hand"))
  (bind _outhit (Class|KismetSystemLibrary|BoxTraceSingleforObjects _returnvalue _returnvalue "5.000000,5.000000,5.000000" (Transformation|GetSocketRotation _mesh "Weapon_Hand") (Utilities|Array|MakeArray "ObjectTypeQuery3") false 0 "ForDuration" true))
  (Utilities|Casting|CastToBP_Survivorll (.HitActor (Collision|BreakHitResult _outhit)))
  (Animation|PlayAnimMontage "/Game/Create/Animation/Killer/Anim_Attack_Delay.Anim_Attack_Delay" 1.5 "None"))