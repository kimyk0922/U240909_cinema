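; BP_Survivor1 is a playable survivor character with Enhanced Input movement, look, a slower walk and hit reactions.
; A killer weapon overlapping the mesh during an attack plays a hit montage through a DoOnce, then sets FirstHit.
; BeginPlay reads SecondHit to choose downed or normal speed and capsule height.
; The item input clears hit flags and resets the DoOnce; nothing here sets SecondHit true.
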(event OnComponentBeginOverlap(Mesh)
  (params (OverlappedComponent :type Primitive%20Component%20Object%20Reference) (OtherActor :type Actor%20Object%20Reference) (OtherComp :type Primitive%20Component%20Object%20Reference) (OtherBodyIndex :type Integer) (bFromSweep :type Boolean) (SweepResult :type Hit%20Result%20Structure%20%28by%20ref%29))
  (bind _asbp_killer_fp (Utilities|Casting|CastToBP_KillerFP OtherActor))
  (if (Variables|/Game/Create/GM/FP/BP_KillerFP.BP_KillerFP_C|GetAttackActionValue _asbp_killer_fp)
    (if (== (Variables|/Game/Create/GM/FP/BP_KillerFP.BP_KillerFP_C|GetSM_Weapon _asbp_killer_fp) OtherComp)
      (Utilities|FlowControl|DoOnce false
        (:Completed
          (Animation|Montage|PlayMontage (Variables|Character|GetMesh) "/Game/Create/Animation/Survivor/Injured_Motion/Anim_Hit.Anim_Hit"
            (:then
              (Variables|Default|SetbFirstHit true))))))))

(event Input|EnhancedActionEvents|EnhancedInputActionIA_item
  (params (ActionValue :type Boolean) (ElapsedSeconds :type Float%20%28double-precision%29) (TriggeredSeconds :type Float%20%28double-precision%29) (InputAction :type Input%20Action%20Object%20Reference :default "/Game/Create/GM/Input/Survivor/IA_item.IA_item"))
  (:Started
    (if (Variables|Default|GetbSecondHit)
      (Variables|Default|SetbSecondHit false)
      (else
        (Variables|Default|SetbFirstHit false)))))

(event Input|EnhancedActionEvents|EnhancedInputActionIA_Walk
  (params (ActionValue :type Boolean) (ElapsedSeconds :type Float%20%28double-precision%29) (TriggeredSeconds :type Float%20%28double-precision%29) (InputAction :type Input%20Action%20Object%20Reference :default "/Game/Create/GM/Input/Survivor/IA_Walk.IA_Walk"))
  (:Ongoing
    (CallFunction|Walk true))
  (:Completed
    (CallFunction|Walk false)))

(event Input|EnhancedActionEvents|EnhancedInputActionIA_item
  (params (ActionValue :type Boolean) (ElapsedSeconds :type Float%20%28double-precision%29) (TriggeredSeconds :type Float%20%28double-precision%29) (InputAction :type Input%20Action%20Object%20Reference :default "/Game/Create/GM/Input/Survivor/IA_item.IA_item"))
  (:Started
    (Variables|Default|SetbFirstHit false)
    (Utilities|FlowControl|DoOnce false) ; enters at Reset
  ))

(event Input|EnhancedActionEvents|EnhancedInputActionIA_Look
  (params (ActionValue :type Vector%202D%20Structure) (ElapsedSeconds :type Float%20%28double-precision%29) (TriggeredSeconds :type Float%20%28double-precision%29) (InputAction :type Input%20Action%20Object%20Reference :default "/Game/Create/GM/Input/Actions/IA_Look.IA_Look"))
  (Pawn|Input|AddControllerYawInput (.x ActionValue))
  (Pawn|Input|AddControllerPitchInput (.y ActionValue)))

(event Input|EnhancedActionEvents|EnhancedInputActionIA_Move
  (params (ActionValue :type Vector%202D%20Structure) (ElapsedSeconds :type Float%20%28double-precision%29) (TriggeredSeconds :type Float%20%28double-precision%29) (InputAction :type Input%20Action%20Object%20Reference :default "/Game/Create/GM/Input/Actions/IA_Move.IA_Move"))
  (bind _returnvalue (Pawn|GetControlRotation :!class /Script/Engine.Pawn))
  (Pawn|Input|AddMovementInput (Math|Vector|GetRightVector (Math|Rotator|MakeRotator (.roll _returnvalue) 0.0 (.yaw _returnvalue))) (.x ActionValue) false)
  (Pawn|Input|AddMovementInput (Math|Vector|GetForwardVector (Math|Rotator|MakeRotator 0.0 0.0 (.yaw (Pawn|GetControlRotation :!class /Script/Engine.Pawn)))) (.y ActionValue) false))

(event EventBeginPlay
  (bind _capsulecomponent (Variables|Collision|GetCapsuleComponent))
  (bind _asplayer_controller (Utilities|Casting|CastToPlayerController (Pawn|GetController)))
  (Utilities|IsValid (PlayerController|LocalPlayerSubsystems|GetEnhancedInputLocalPlayerSubsystem _asplayer_controller)
    (:Is%20Valid
      (Input|AddMappingContext (PlayerController|LocalPlayerSubsystems|GetEnhancedInputLocalPlayerSubsystem _asplayer_controller) "/Game/Create/GM/Input/IMC_Survivor.IMC_Survivor" 0 "(bIgnoreAllPressedKeysUntilRelease=True,bForceImmediately=False,bNotifyUserSettings=False)")
      (if (Variables|Default|GetbSecondHit)
        (CallFunction|Down true)
        (Components|Capsule|SetCapsuleSize _capsulecomponent 34.0 44.0 true)
        (else
          (CallFunction|Down false)
          (Components|Capsule|SetCapsuleSize _capsulecomponent 34.0 88.0 true))))))

(fn ConstructionScript)

(fn Walk
  (params (bWalk :type Boolean))
  (bind _charactermovement (Variables|Character|GetCharacterMovement))
  (if bWalk
    (Variables|/Script/Engine.CharacterMovementComponent|SetMaxWalkSpeed _charactermovement 3e+02)
    (else
      (Variables|/Script/Engine.CharacterMovementComponent|SetMaxWalkSpeed _charactermovement 6e+02))))

(fn Down
  (params (Down :type Boolean))
  (bind _charactermovement (Variables|Character|GetCharacterMovement))
  (if Down
    (Variables|/Script/Engine.CharacterMovementComponent|SetMaxWalkSpeed _charactermovement 1.5e+02)
    (else
      (Variables|/Script/Engine.CharacterMovementComponent|SetMaxWalkSpeed _charactermovement 6e+02))))