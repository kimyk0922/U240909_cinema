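; Survivor player character for a killer-versus-survivor game, with Enhanced Input movement, look and a slower walk toggle.
; HitMotion runs a two-stage injury, a hit montage then a down montage that activates the Box, while the item input clears one stage.
; It registers itself with BP_Killerll, reports Box overlaps to it, and Detach drops it in front of the killer.
; The downed speed and capsule resize logic is unconnected.
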(event OnComponentBeginOverlap(Box)
  (params (OverlappedComponent :type Primitive%20Component%20Object%20Reference) (OtherActor :type Actor%20Object%20Reference) (OtherComp :type Primitive%20Component%20Object%20Reference) (OtherBodyIndex :type Integer) (bFromSweep :type Boolean) (SweepResult :type Hit%20Result%20Structure%20%28by%20ref%29))
  (bind _asbp_killerll (Utilities|Casting|CastToBP_Killerll OtherActor))
  (Default|EvtBeginOverlapEventSurvivor _asbp_killerll self))

(event OnComponentEndOverlap(Box)
  (params (OverlappedComponent :type Primitive%20Component%20Object%20Reference) (OtherActor :type Actor%20Object%20Reference) (OtherComp :type Primitive%20Component%20Object%20Reference) (OtherBodyIndex :type Integer))
  (bind _asbp_killerll (Utilities|Casting|CastToBP_Killerll OtherActor))
  (Default|EvtEndOverlapEventSurvivor _asbp_killerll self))

(event Custom|HitMotion
  (if (Variables|Default|GetbFirstHit)
    (Development|PrintString (Utilities|String|ToString(Boolean) (Variables|Default|GetbFirstHit)) true true "(R=0.000000,G=0.000000,B=1.000000,A=1.000000)" 1e+01)
    (Animation|Montage|PlayMontage (Variables|Character|GetMesh) "/Game/Create/Animation/Anim_Down.Anim_Down"
      (:then
        (bind _output_get (Variables|Default|SetbSecondHit true))
        (Components|Activation|SetActive (Variables|Default|GetBox) _output_get false)))
    (else
      (Development|PrintString (Utilities|String|ToString(Boolean) (Variables|Default|GetbFirstHit)) true true "(R=1.000000,G=0.000000,B=0.000000,A=1.000000)" 1e+01)
      (Animation|Montage|PlayMontage (Variables|Character|GetMesh) "/Game/Create/Animation/Survivor/Injured_Motion/Anim_Hit.Anim_Hit"
        (:then
          (Variables|Default|SetbFirstHit true))))))

(event Custom|RosOffWalk
  (CallFunction|Walk false))

(event Custom|RosWalk
  (CallFunction|Walk true))

(event Input|EnhancedActionEvents|EnhancedInputActionIA_item
  (params (ActionValue :type Boolean) (ElapsedSeconds :type Float%20%28double-precision%29) (TriggeredSeconds :type Float%20%28double-precision%29) (InputAction :type Input%20Action%20Object%20Reference :default "/Game/Create/GM/Input/Survivor/IA_item.IA_item"))
  (:Started
    (if (Variables|Default|GetbSecondHit)
      (Variables|Default|SetbSecondHit false)
      (else
        (Variables|Default|SetbFirstHit false)))))

(event Input|EnhancedActionEvents|EnhancedInputActionIA_Walk
  (params (ActionValue :type Boolean) (ElapsedSeconds :type Float%20%28double-precision%29) (TriggeredSeconds :type Float%20%28double-precision%29) (InputAction :type Input%20Action%20Object%20Reference :default "/Game/Create/GM/Input/Survivor/IA_Walk.IA_Walk"))
  (:Started
    (CallFunction|RosWalk))
  (:Completed
    (CallFunction|RosOffWalk)))

(event Input|EnhancedActionEvents|EnhancedInputActionIA_Look
  (params (ActionValue :type Vector%202D%20Structure) (ElapsedSeconds :type Float%20%28double-precision%29) (TriggeredSeconds :type Float%20%28double-precision%29) (InputAction :type Input%20Action%20Object%20Reference :default "/Game/Create/GM/Input/Actions/IA_Look.IA_Look"))
  (Pawn|Input|AddControllerYawInput (.x ActionValue))
  (Pawn|Input|AddControllerPitchInput (.y ActionValue)))

(event Input|EnhancedActionEvents|EnhancedInputActionIA_Move
  (params (ActionValue :type Vector%202D%20Structure) (ElapsedSeconds :type Float%20%28double-precision%29) (TriggeredSeconds :type Float%20%28double-precision%29) (InputAction :type Input%20Action%20Object%20Reference :default "/Game/Create/GM/Input/Actions/IA_Move.IA_Move"))
  (bind _returnvalue (Pawn|GetControlRotation :!class /Script/Engine.Pawn))
  (Pawn|Input|AddMovementInput (Math|Vector|GetRightVector (Math|Rotator|MakeRotator (.roll _returnvalue) 0.0 (.yaw _returnvalue))) (.x ActionValue) false)
  (Pawn|Input|AddMovementInput (Math|Vector|GetForwardVector (Math|Rotator|MakeRotator 0.0 0.0 (.yaw (Pawn|GetControlRotation :!class /Script/Engine.Pawn)))) (.y ActionValue) false))

(event Game|Damage|EventAnyDamage
  (params (Damage :type Float%20%28single-precision%29) (DamageType :type Damage%20Type%20Object%20Reference) (InstigatedBy :type Controller%20Object%20Reference) (DamageCauser :type Actor%20Object%20Reference)))

(event EventBeginPlay
  (bind _asplayer_controller (Utilities|Casting|CastToPlayerController (Pawn|GetController)))
  (Utilities|IsValid (PlayerController|LocalPlayerSubsystems|GetEnhancedInputLocalPlayerSubsystem _asplayer_controller)
    (:Is%20Valid
      (Input|AddMappingContext (PlayerController|LocalPlayerSubsystems|GetEnhancedInputLocalPlayerSubsystem _asplayer_controller) "/Game/Create/GM/Input/IMC_Survivor.IMC_Survivor" 0 "(bIgnoreAllPressedKeysUntilRelease=True,bForceImmediately=False,bNotifyUserSettings=False)")
      (bind _returnvalue (Actor|GetActorOfClass "/Game/Create/GM/BP_Killerll.BP_Killerll_C"))
      (Variables|/Game/Create/GM/BP_Killerll.BP_Killerll_C|SetSurvivor _returnvalue self))))

(fn ConstructionScript)

(fn Walk
  (params (bWalk :type Boolean))
  (bind _charactermovement (Variables|Character|GetCharacterMovement))
  (if bWalk
    (Variables|/Script/Engine.CharacterMovementComponent|SetMaxWalkSpeed _charactermovement 3e+02)
    (else
      (Variables|/Script/Engine.CharacterMovementComponent|SetMaxWalkSpeed _charactermovement 6e+02))))

(fn Down
  (params (Down :type Boolean))
  (bind _charactermovement (Variables|Character|GetCharacterMovement))
  (if Down
    (Variables|/Script/Engine.CharacterMovementComponent|SetMaxWalkSpeed _charactermovement 1.5e+02)
    (else
      (Variables|/Script/Engine.CharacterMovementComponent|SetMaxWalkSpeed _charactermovement 6e+02))))

(fn Detach
  (bind _killer (Variables|Default|GetKiller))
  (Transformation|DetachFromActor self "KeepRelative" "KeepRelative" "KeepRelative")
  (Transformation|SetActorLocation self (+ (Transformation|GetActorLocation _killer) (* (Transformation|GetActorForwardVector _killer) 1e+02)) false false)
  (Variables|/Game/Create/GM/BP_Killerll.BP_Killerll_C|SetGrabToSurvivor _killer false))