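; Exit gate actor that a survivor opens by holding the trigger input at its lever.
; Box overlap with a survivor shows a prompt widget and opens a Gate that lets the ongoing input through, received via player controller 0.
; Each input tick rotates the socket-attached handle and gear and raises a counter.
; At the threshold, a looping timer slides three door pieces in sequence, third to first, by fixed offset steps.
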(event OnComponentBeginOverlap(Box)
  (params (OverlappedComponent :type Primitive%20Component%20Object%20Reference) (OtherActor :type Actor%20Object%20Reference) (OtherComp :type Primitive%20Component%20Object%20Reference) (OtherBodyIndex :type Integer) (bFromSweep :type Boolean) (SweepResult :type Hit%20Result%20Structure%20%28by%20ref%29))
  (bind _asbp_survivorll (Utilities|Casting|CastToBP_Survivorll OtherActor))
  (bind _returnvalue (UserInterface|CreateWidget "/Game/Create/Widget/WG_Trigger_Info.WG_Trigger_Info_C" (Game|GetPlayerController (Variables|/Script/Engine.Pawn|GetPlayerState _asbp_survivorll))))
  (UserInterface|Viewport|AddtoPlayerScreen _returnvalue)
  (Utilities|FlowControl|Gate true) ; enters at Open
)

(event OnComponentEndOverlap(Box)
  (params (OverlappedComponent :type Primitive%20Component%20Object%20Reference) (OtherActor :type Actor%20Object%20Reference) (OtherComp :type Primitive%20Component%20Object%20Reference) (OtherBodyIndex :type Integer))
  (Utilities|Casting|CastToBP_Survivorll OtherActor)
  (Widget|RemovefromParent (stale OnComponentBeginOverlap(Box) _returnvalue))
  (Utilities|FlowControl|Gate true) ; enters at Close
)

(event Input|EnhancedActionEvents|EnhancedInputActionIA_Live_Trigger
  (params (ActionValue :type Boolean) (ElapsedSeconds :type Float%20%28double-precision%29) (TriggeredSeconds :type Float%20%28double-precision%29) (InputAction :type Input%20Action%20Object%20Reference :default "/Game/Create/GM/Input/Survivor/IA_Live_Trigger.IA_Live_Trigger"))
  (:Ongoing
    (Utilities|FlowControl|Gate true
      (:Exit
        (bind _result (CallFunction|Action))
        (Development|PrintString (Utilities|String|ToString(Float) _result))
        (if (> _result 89.0)
          (Utilities|Time|SetTimerbyFunctionName 0 "DoorOpen" 0.05 true))))))

(event EventBeginPlay
  (Input|EnableInput (Game|GetPlayerController 0)))

(fn ConstructionScript
  (Transformation|AttachComponentToComponent (Variables|Default|GetSM_Exit_Lever_Handle) (Variables|Default|GetSM_Exit_Lever_Body) "Handle" "SnapToTarget" "SnapToTarget" "SnapToTarget" true)
  (Transformation|AttachComponentToComponent (Variables|Default|GetSM_Exit_Gear) (Variables|Default|GetSM_Exit_Top) "Gear" "SnapToTarget" "SnapToTarget" "SnapToTarget" true))

(fn Action
  (if (< (Variables|Default|GetActionValue) 9e+01)
    (Transformation|AddLocalRotation (Variables|Default|GetSM_Exit_Lever_Handle) "0.000000,0.000000,-2.000000" false false)
    (Transformation|AddLocalRotation (Variables|Default|GetSM_Exit_Gear) "2.000000,0.000000,0.000000" false false)
    (bind _result (Math|Float|IncrementFloat (Variables|Default|GetActionValue))
      (:%20%20
        (return _result)))))

(fn DoorOpen
  (if (< (Variables|Default|GetDoor03) 52.0)
    (Transformation|AddLocalOffset (Variables|Default|GetSM_Exit_Door_03) "-6.000000,0.000000,0.000000" false false)
    (Math|Float|IncrementFloat (Variables|Default|GetDoor03))
    (elif (< (Variables|Default|GetDoor02) 52.0)
      (Transformation|AddLocalOffset (Variables|Default|GetSM_Exit_Door_02) "-6.000000,0.000000,0.000000" false false)
      (Math|Float|IncrementFloat (Variables|Default|GetDoor02))
      (elif (< (Variables|Default|GetDoor01) 52.0)
        (Transformation|AddLocalOffset (Variables|Default|GetSM_Exit_Door_01) "-6.000000,0.000000,0.000000" false false)
        (Math|Float|IncrementFloat (Variables|Default|GetDoor01))))))