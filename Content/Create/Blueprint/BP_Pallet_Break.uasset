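; A droppable, breakable pallet for a Survivor-versus-Killer game with per-player prompts.
; A timeline, started by gated survivor input or a Killer entering Box1, tilts the pallet and flags an overlapping Killer to react.
; Once dropped, a second gate lets the Killer play a destroy montage with input disabled, then destroys the actor.
; Functions exposing two-stage physics breakup of the mesh pieces are not called within this Blueprint.
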(event OnComponentBeginOverlap(Box)
  (params (OverlappedComponent :type Primitive%20Component%20Object%20Reference) (OtherActor :type Actor%20Object%20Reference) (OtherComp :type Primitive%20Component%20Object%20Reference) (OtherBodyIndex :type Integer) (bFromSweep :type Boolean) (SweepResult :type Hit%20Result%20Structure%20%28by%20ref%29))
  (bind _returnvalue (Game|GetPlayerController 0))
  ;[0 0.2 0 0.5 15] Surviver
  (bind _asbp_survivorll (Utilities|Casting|CastToBP_Survivorll OtherActor)
    (:then
      (Variables|/Game/Create/GM/BP_Survivorll.BP_Survivorll_C|SetCurrPallet _asbp_survivorll self)
      (bind _returnvalue_2 (UserInterface|CreateWidget "/Game/Create/Widget/WG_Trigger_Info.WG_Trigger_Info_C"))
      (UserInterface|Viewport|AddtoPlayerScreen _returnvalue_2 1)
      (Utilities|FlowControl|Gate true) ; enters at Open
    )
    (:CastFailed
      (if (Variables|Default|GetbIsPalletPlay)
        ;[0.2 0 0 0.5 15] Killer
        (bind _asbp_killerll (Utilities|Casting|CastToBP_Killerll OtherActor))
        (bind _output_get (Variables|Default|SetKiller _asbp_killerll))
        (Variables|/Game/Create/GM/BP_Killerll.BP_Killerll_C|SetCurrPallet _output_get self)
        (bind _returnvalue_3 (UserInterface|CreateWidget "/Game/Create/Widget/WG_Trigger_Info.WG_Trigger_Info_C"))
        (UserInterface|Viewport|AddtoPlayerScreen _returnvalue_3)
        (Utilities|FlowControl|Gate true) ; enters at Open
      ))))

(event OnComponentEndOverlap(Box)
  (params (OverlappedComponent :type Primitive%20Component%20Object%20Reference) (OtherActor :type Actor%20Object%20Reference) (OtherComp :type Primitive%20Component%20Object%20Reference) (OtherBodyIndex :type Integer))
  (bind _returnvalue (Game|GetPlayerController 0))
  ;[0 0.2 0 0.5 15] Surviver
  (Utilities|Casting|CastToBP_Survivorll OtherActor
    (:then
      (Widget|RemovefromParent (stale OnComponentBeginOverlap(Box) _returnvalue_2))
      (Utilities|FlowControl|Gate true) ; enters at Close
    )
    (:CastFailed
      ;[0.2 0 0 0.5 15] Killer
      (if (Variables|Default|GetbIsPalletPlay)
        (bind _asbp_killerll (Utilities|Casting|CastToBP_Killerll OtherActor))
        (bind _output_get (Variables|Default|SetKiller _asbp_killerll))
        (Utilities|IsValid _output_get
          (:Is%20Valid
            (Widget|RemovefromParent (stale OnComponentBeginOverlap(Box) _returnvalue_3))
            (Utilities|FlowControl|Gate true) ; enters at Close
          ))))))

(event OnComponentBeginOverlap(Box1)
  (params (OverlappedComponent :type Primitive%20Component%20Object%20Reference) (OtherActor :type Actor%20Object%20Reference) (OtherComp :type Primitive%20Component%20Object%20Reference) (OtherBodyIndex :type Integer) (bFromSweep :type Boolean) (SweepResult :type Hit%20Result%20Structure%20%28by%20ref%29))
  ;[0 0.2 0 0.5 15] Surviver
  (bind _asbp_killerll (Utilities|Casting|CastToBP_Killerll OtherActor))
  (bind _movespeed (Timeline|PalletMotion Play)
    (:Update
      (Transformation|SetRelativeRotation (Variables|Default|GetPallet_Bone) (Math|Rotator|MakeRotator 0.0 (Math|Float|Lerp 0.0 45.0 _movespeed) 0.0) false false)
      (if (Collision|IsOverlappingActor (Variables|Default|GetBox1) _asbp_killerll :!class /Script/Engine.PrimitiveComponent)
        (Variables|/Game/Create/GM/BP_Killerll.BP_Killerll_C|SetPallet_React _asbp_killerll true)
        (Variables|Default|SetbIsPalletPlay true)
        (Components|DestroyComponent (Variables|BP_Pallet_Break_C|GetBox1 (Variables|Default|GetPallet)))
        (else
          (Variables|Default|SetbIsPalletPlay true))))))

(event Input|EnhancedActionEvents|EnhancedInputActionIA_Killer_Trigger
  (params (ActionValue :type Boolean) (ElapsedSeconds :type Float%20%28double-precision%29) (TriggeredSeconds :type Float%20%28double-precision%29) (InputAction :type Input%20Action%20Object%20Reference :default "/Game/Create/GM/Input/Killer/IA_Killer_Trigger.IA_Killer_Trigger"))
  (bind _returnvalue (Game|GetPlayerController 0))
  (bind _killer (Variables|Default|GetKiller))
  ;[0.2 0 0 0.5 15] Killer
  (:Started
    (Utilities|FlowControl|Gate true
      (:Exit
        (Animation|Montage|PlayMontage (Variables|/Script/Engine.Character|GetMesh (stale OnComponentBeginOverlap(Box) _output_get)) "/Game/Create/Animation/Killer/Anim_Destroy.Anim_Destroy"
          (:then
            (Input|DisableInput _killer _returnvalue))
          (:OnCompleted
            (Input|EnableInput _killer _returnvalue)
            (Actor|DestroyActor)))))))

(event Input|EnhancedActionEvents|EnhancedInputActionIA_Live_Trigger
  (params (ActionValue :type Boolean) (ElapsedSeconds :type Float%20%28double-precision%29) (TriggeredSeconds :type Float%20%28double-precision%29) (InputAction :type Input%20Action%20Object%20Reference :default "/Game/Create/GM/Input/Survivor/IA_Live_Trigger.IA_Live_Trigger"))
  ;[0 0.2 0 0.5 15] Surviver
  (:Started
    (Utilities|FlowControl|Gate true
      (:Exit
        (bind _movespeed (Timeline|PalletMotion Play)
          (:Update
            (Transformation|SetRelativeRotation (Variables|Default|GetPallet_Bone) (Math|Rotator|MakeRotator 0.0 (Math|Float|Lerp 0.0 45.0 _movespeed) 0.0) false false)
            (if (Collision|IsOverlappingActor (Variables|Default|GetBox1) (stale OnComponentBeginOverlap(Box1) _asbp_killerll) :!class /Script/Engine.PrimitiveComponent)
              (Variables|/Game/Create/GM/BP_Killerll.BP_Killerll_C|SetPallet_React (stale OnComponentBeginOverlap(Box1) _asbp_killerll) true)
              (Variables|Default|SetbIsPalletPlay true)
              (Components|DestroyComponent (Variables|BP_Pallet_Break_C|GetBox1 (Variables|Default|GetPallet)))
              (else
                (Variables|Default|SetbIsPalletPlay true)))))))))

(event EventBeginPlay
  ;[0.2 0 0 0.5 15] Killer
  (Input|EnableInput (Game|GetPlayerController 0))
  (bind _returnvalue (Actor|GetActorOfClass "BP_Pallet_Break_C"))
  (Variables|BP_Pallet_Break_C|SetPallet _returnvalue self))

(fn ConstructionScript)

(fn SimulatePhysics
  (params (bSimulate :type Boolean))
  (for _array_element (Components|GetChildrenComponents (Variables|BP_Pallet_Break_C|GetBox (Variables|Default|GetPallet)) false)
    (bind _asstatic_mesh_component (Utilities|Casting|CastToStaticMeshComponent _array_element))
    (Physics|SetSimulatePhysics _asstatic_mesh_component bSimulate)))

(fn SetPhysicsSecondTarget
  (Physics|SetSimulatePhysics (Variables|Default|GetPallet_Sphere_024) true))

(fn SetDestroySecondAction
  (CallFunction|SetPhysicsSecondTarget))

(fn SetDestroyFirstAction
  (CallFunction|SetPhysicsFirstTarget))

(fn SetPhysicsFirstTarget
  (Physics|SetSimulatePhysics (Variables|Default|GetPallet_Cube_044) true))