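; Pallet obstacle that a survivor drops and the killer then breaks.
; Box overlap picks the role from IsPalletPlay, showing the locally controlled player a prompt and gating input that fires play or destroy dispatchers.
; RepNotifies tilt the pallet bone on a looping timer and play the killer's break montage.
; Destroy functions, not called here, release hand-picked pieces to physics in two stages.
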(event OnComponentBeginOverlap(Box)
  (params (OverlappedComponent :type Primitive%20Component%20Object%20Reference) (OtherActor :type Actor%20Object%20Reference) (OtherComp :type Primitive%20Component%20Object%20Reference) (OtherBodyIndex :type Integer) (bFromSweep :type Boolean) (SweepResult :type Hit%20Result%20Structure%20%28by%20ref%29))
  ;[0 0.2 0 0.5 15] Surviver
  (if (Variables|Default|GetbIsPalletPlay)
    (bind _asbp_killer_fptest (Utilities|Casting|CastToBP_KillerFPTest (stale OnComponentEndOverlap(Box) OtherActor)))
    (bind _output_get (Variables|Default|SetKiller _asbp_killer_fptest))
    (Variables|/Game/DK/BP_KillerFPTest.BP_KillerFPTest_C|SetCurrPallet _output_get self)
    (if (Pawn|IsLocallyControlled (Variables|Default|GetKiller))
      (Input|EnableInput (Pawn|GetLocalViewingPlayerController (Variables|Default|GetKiller)))
      (bind _returnvalue (Game|ConstructObjectfromClass "/Game/Create/Widget/WG_Trigger_Info.WG_Trigger_Info_C"))
      (bind _output_get_2 (Variables|Default|SetWidget%20REF _returnvalue))
      (UserInterface|Viewport|AddtoViewport _output_get_2 0)
      (Utilities|FlowControl|Gate true) ; enters at Open
    )
    (else
      (bind _asbp_test_survivor (Utilities|Casting|CastToBP_TestSurvivor OtherActor))
      (bind _output_get_3 (Variables|Default|SetCurrent%20Survivor _asbp_test_survivor))
      (Variables|/Game/DK/BP_TestSurvivor.BP_TestSurvivor_C|SetCurrentPallet _output_get_3 self)
      (if (Pawn|IsLocallyControlled (Variables|Default|GetCurrent%20Survivor))
        (Input|EnableInput (Pawn|GetLocalViewingPlayerController (Variables|Default|GetCurrent%20Survivor)))
        (bind _returnvalue_2 (Game|ConstructObjectfromClass "/Game/Create/Widget/WG_Trigger_Info.WG_Trigger_Info_C"))
        (bind _output_get_4 (Variables|Default|SetWidget%20REF _returnvalue_2))
        (UserInterface|Viewport|AddtoViewport _output_get_4 0)
        (Utilities|FlowControl|Gate true) ; enters at Open
      ))))

(event OnComponentEndOverlap(Box)
  (params (OverlappedComponent :type Primitive%20Component%20Object%20Reference) (OtherActor :type Actor%20Object%20Reference) (OtherComp :type Primitive%20Component%20Object%20Reference) (OtherBodyIndex :type Integer))
  ;[0 0.2 0 0.5 15] Surviver
  (if (Variables|Default|GetbIsPalletPlay)
    (bind _asbp_killer_fptest (Utilities|Casting|CastToBP_KillerFPTest OtherActor))
    (bind _output_get (Variables|Default|SetKiller _asbp_killer_fptest))
    (Variables|/Game/DK/BP_KillerFPTest.BP_KillerFPTest_C|SetCurrPallet _output_get self)
    (if (Pawn|IsLocallyControlled (Variables|Default|GetKiller))
      (Input|DisableInput (Pawn|GetLocalViewingPlayerController (Variables|Default|GetKiller)))
      (bind _widget_ref (Variables|Default|GetWidget%20REF)
        (:then
          (Widget|RemovefromParent _widget_ref)
          (Utilities|FlowControl|Gate true) ; enters at Close
        )
        (:else)))
    (else
      (bind _asbp_test_survivor (Utilities|Casting|CastToBP_TestSurvivor OtherActor))
      (bind _output_get_2 (Variables|Default|SetCurrent%20Survivor _asbp_test_survivor))
      (Variables|/Game/DK/BP_TestSurvivor.BP_TestSurvivor_C|SetCurrentPallet _output_get_2 self)
      (if (Pawn|IsLocallyControlled (Variables|Default|GetCurrent%20Survivor))
        (Input|DisableInput (Pawn|GetLocalViewingPlayerController (Variables|Default|GetCurrent%20Survivor)))
        (bind _widget_ref_2 (Variables|Default|GetWidget%20REF)
          (:then
            (Widget|RemovefromParent _widget_ref_2)
            (Utilities|FlowControl|Gate true) ; enters at Close
          )
          (:else))))))

(event Input|EnhancedActionEvents|EnhancedInputActionIA_Killer_Trigger
  (params (ActionValue :type Boolean) (ElapsedSeconds :type Float%20%28double-precision%29) (TriggeredSeconds :type Float%20%28double-precision%29) (InputAction :type Input%20Action%20Object%20Reference :default "/Game/Create/GM/Input/Killer/IA_Killer_Trigger.IA_Killer_Trigger"))
  (:Started
    (Utilities|FlowControl|Gate true
      (:Exit
        (bind _widget_ref (Variables|Default|GetWidget%20REF)
          (:then
            (Widget|RemovefromParent _widget_ref)
            (Default|CallEDPalletDestroy self))
          (:else))))))

(event Input|EnhancedActionEvents|EnhancedInputActionIA_Live_Trigger
  (params (ActionValue :type Boolean) (ElapsedSeconds :type Float%20%28double-precision%29) (TriggeredSeconds :type Float%20%28double-precision%29) (InputAction :type Input%20Action%20Object%20Reference :default "/Game/Create/GM/Input/Survivor/IA_Live_Trigger.IA_Live_Trigger"))
  (:Started
    (Utilities|FlowControl|Gate true
      (:Exit
        (Default|CallEDPalletPlay self)))))

(fn ConstructionScript)

(fn SimulatePhysics
  (params (bSimulate :type Boolean))
  (for _array_element (Components|GetChildrenComponents (Variables|BP_Pallet_Break_DK_C|GetBox (Variables|Default|GetPallet)) false)
    (bind _asstatic_mesh_component (Utilities|Casting|CastToStaticMeshComponent _array_element))
    (Physics|SetSimulatePhysics _asstatic_mesh_component bSimulate)))

(fn SetPhysicsSecondTarget
  (Physics|SetSimulatePhysics (Variables|Default|GetPallet_Sphere_024) true))

(fn SetDestroySecondAction
  (CallFunction|SetPhysicsSecondTarget))

(fn SetDestroyFirstAction
  (CallFunction|SetPhysicsFirstTarget))

(fn SetPhysicsFirstTarget
  (Physics|SetSimulatePhysics (Variables|Default|GetPallet_Cube_044) true))

(fn OnRepBIsPalletPlay
  (Utilities|Time|SetTimerbyFunctionName 0 "RotatePallet" 0.01 true)
  (bind _widget_ref (Variables|Default|GetWidget%20REF)
    (:then
      (Widget|RemovefromParent _widget_ref))
    (:else)))

(fn RotatePallet
  (Transformation|SetRelativeRotation (Variables|Default|GetPallet_Bone) (Math|Rotator|MakeRotator 0.0 (Variables|Default|GetRotateRate) 0.0) false false)
  (bind _output_get (Variables|Default|SetRotateRate (+ (Variables|Default|GetRotateRate) 2.0)))
  (if (> _output_get 45.0)
    (Utilities|Time|ClearTimerbyFunctionName 0 "RotatePallet")))

(fn OnRepBIsPalletDestroy
  (bind _killer (Variables|Default|GetKiller))
  (Animation|PlayAnimMontage (Variables|Default|GetKiller) "/Game/Create/Animation/Killer/Anim_Destroy.Anim_Destroy" 1.0 "None")
  (Input|DisableInput _killer (Pawn|GetLocalViewingPlayerController _killer)))