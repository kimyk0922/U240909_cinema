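; BP_ExitTest is an exit gate with a hand lever, a gear and three sliding doors, its meshes snapped to sockets at construction.
; Each Action call turns the handle and gear and advances ActionValue toward a cap, returning the count.
; DoorOpen, a timer callback started outside these graphs, slides doors 03, 02 and 01 open in sequence by stepped offsets, then prints a clear message and stops its timer.
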(fn ConstructionScript
  (Transformation|AttachComponentToComponent (Variables|Default|GetSM_Exit_Lever_Handle) (Variables|Default|GetSM_Exit_Lever_Body) "Handle" "SnapToTarget" "SnapToTarget" "SnapToTarget" true)
  (Transformation|AttachComponentToComponent (Variables|Default|GetSM_Exit_Gear) (Variables|Default|GetSM_Exit_Top) "Gear" "KeepRelative" "SnapToTarget" "SnapToTarget" true))

(fn Action
  (if (< (Variables|Default|GetActionValue) 7.2e+02)
    (Transformation|AddLocalRotation (Variables|Default|GetSM_Exit_Lever_Handle) "0.000000,0.000000,-2.000000" false false)
    (Transformation|AddLocalRotation (Variables|Default|GetSM_Exit_Gear) "-0.200000,0.000000,0.000000" false false)
    (bind _result (Math|Float|IncrementFloat (Variables|Default|GetActionValue))
      (:%20%20
        (return _result)))))

(fn DoorOpen
  (if (< (Variables|Default|GetDoor03) 52.0)
    (Transformation|AddLocalOffset (Variables|Default|GetSM_Exit_Door_03) "-6.000000,0.000000,0.000000" false false)
    (Math|Float|IncrementFloat (Variables|Default|GetDoor03))
    (elif (< (Variables|Default|GetDoor02) 52.0)
      (Transformation|AddLocalOffset (Variables|Default|GetSM_Exit_Door_02) "-6.000000,0.000000,0.000000" false false)
      (Math|Float|IncrementFloat (Variables|Default|GetDoor02))
      (elif (< (Variables|Default|GetDoor01) 52.0)
        (Transformation|AddLocalOffset (Variables|Default|GetSM_Exit_Door_01) "-6.000000,0.000000,0.000000" false false)
        (Math|Float|IncrementFloat (Variables|Default|GetDoor01))
        (else
          (Development|PrintString "Clear~!~!")
          (Utilities|Time|ClearTimerbyFunctionName 0 "DoorOpen"))))))