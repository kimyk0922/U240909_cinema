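; BP_LockerTest is a test locker that a BP_TestSurvivor can hide in.
; Its Box overlap stores the survivor and toggles the locker's input, so pressing Q passes the locker to the survivor's CallCallhideonbush.
; ToggleHide flips the character's visibility and collision and blends the camera between locker and character.
; The event graph's own ToggleHide call and door timeline are disconnected leftovers.
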(event OnComponentBeginOverlap(Box)
  (params (OverlappedComponent :type Primitive%20Component%20Object%20Reference) (OtherActor :type Actor%20Object%20Reference) (OtherComp :type Primitive%20Component%20Object%20Reference) (OtherBodyIndex :type Integer) (bFromSweep :type Boolean) (SweepResult :type Hit%20Result%20Structure%20%28by%20ref%29))
  (bind _asbp_test_survivor (Utilities|Casting|CastToBP_TestSurvivor OtherActor))
  (Variables|Default|SetTestSurvivor _asbp_test_survivor)
  (Input|EnableInput (Pawn|GetLocalViewingPlayerController (Variables|Default|GetTestSurvivor))))

(event OnComponentEndOverlap(Box)
  (params (OverlappedComponent :type Primitive%20Component%20Object%20Reference) (OtherActor :type Actor%20Object%20Reference) (OtherComp :type Primitive%20Component%20Object%20Reference) (OtherBodyIndex :type Integer))
  (Utilities|Casting|CastToBP_TestSurvivor OtherActor)
  (Input|DisableInput (Pawn|GetLocalViewingPlayerController (Variables|Default|GetTestSurvivor)))
  (Variables|Default|SetIsClicked? false))

(event Input|KeyboardEvents|Q
  (params (Key :type Key%20Structure :default "None"))
  (:Pressed
    (Default|CallCallhideonbush (Variables|Default|GetTestSurvivor) self)))

(fn ConstructionScript)

(fn ToggleHide
  (params (NewParam :type BP%20Test%20Survivor%20Object%20Reference))
  (bind _returnvalue (Pawn|GetController NewParam))
  (bind _asbp_pc (Utilities|Casting|CastToBP_PC _returnvalue))
  (if (Variables|Default|GetIsHide?)
    (Variables|Default|SetIsHide? false)
    (Rendering|SetActorHiddenInGame NewParam false)
    (Collision|SetActorEnableCollision NewParam true)
    (Game|Player|SetViewTargetwithBlend _asbp_pc NewParam 0.3 "VTBlend_Linear" 0.0 false)
    (else
      (Variables|Default|SetIsHide? true)
      (Rendering|SetActorHiddenInGame NewParam true)
      (Collision|SetActorEnableCollision NewParam false)
      (Game|Player|SetViewTargetwithBlend _asbp_pc self 0.3 "VTBlend_Linear" 0.0 false))))